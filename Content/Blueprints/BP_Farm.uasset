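; BP_Farm is a clickable farm building that finishes construction over time, then accumulates product up to a capacity randomized at BeginPlay.
; Tick drives UpdateBuilding, which counts down build time and then swaps in the Farm mesh.
; Tick also calls UpdateProduction, whose Delay paces additions of Power to Product, clamped at Capacity and skipped during construction.
; Clicking the mesh assigns this farm to the first BP_Farm_State widget found.
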(event OnClicked(Farm_Mesh)
  (params (TouchedComponent :type Primitive%20Component%20Object%20Reference) (ButtonPressed :type Key%20Structure :default "None"))
  (bind _foundwidgets (Widget|GetAllWidgetsOfClass "/Game/Widgets/BP_Farm_State.BP_Farm_State_C" false))
  (Variables|/Game/Widgets/BP_Farm_State.BP_Farm_State_C|SetRef_Farm (Utilities|Array|Get(acopy) _foundwidgets) self))

(event EventBeginPlay
  (Variables|Production|SetCapacity (Math|Random|RandomIntegerinRange 30 100)))

(event EventTick
  (params (DeltaSeconds :type Float%20%28single-precision%29))
  (if (Variables|Building|GetIsBuilding)
    (Utilities|UpdateBuilding DeltaSeconds
      (:End
        _)))
  (Utilities|UpdateProduction))

(fn ConstructionScript)